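; BP_Ability is an ability actor that starts casting as soon as it spawns.
; BeginPlay gets the HUD from the ThirdPersonGameMode, then BeginCasting shows a cast bar if the cast time is above zero and binds to its success event.
; CastAbility is a print-only placeholder, and InteruptCasting prints and destroys the actor.
; Zero-cast-time abilities have no handling yet.
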(event `self.ReceiveBeginPlay`
  (bind _asthird_person_game_mode (cast `/Game/ThirdPersonBP/Blueprints/ThirdPersonGameMode` (`GameplayStatics.GetGameMode`)))
  (set `self.HUD UI` (`/Game/ThirdPersonBP/Blueprints/ThirdPersonGameMode.HeadsUpDisplay` _asthird_person_game_mode))
  (`self.BeginCasting`))

(fn `BeginCasting`
  (bind (_abilitydetails_name _abilitydetails_description _abilitydetails_cost _abilitydetails_cooldown _abilitydetails_casttime) (break `/Game/AbilitySystem/SAbilityDetails` (`self.AbilityDetails`)))
  (if (> _abilitydetails_casttime 0.0)
    (bind _castbar (`/Game/AbilitySystem/UI/WBP_HeadsUpDisplay.DisplayCastBar` (`self.HUD UI`) self))
    (add `/Game/AbilitySystem/UI/WBP_CastBar.CastSuccessful` _castbar (`|CreateDelegate` :!event `CastAbility`))))

(fn `CastAbility`
  (`KismetSystemLibrary.PrintString` "cast ability"))

(fn `InteruptCasting`
  (`KismetSystemLibrary.PrintString` "interrupt casting")
  (`self.K2_DestroyActor`))

(fn `UserConstructionScript`)